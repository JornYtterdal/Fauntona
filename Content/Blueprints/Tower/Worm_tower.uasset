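; Worm tower turret that targets an actor entering its trigger and fires Probe_BP at it.
; Trigger overlaps set the target and toggle targeting, with no actor filtering, so any exit clears it.
; While targeting, Tick aims the gun with clamped pitch and spawns probes at the BarrelEnd socket, paced by a short Delay.
; Otherwise it levels the gun and slowly spins it in yaw.
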(event OnComponentBeginOverlap(trigger)
  (params (OverlappedComponent :type Primitive%20Component%20Object%20Reference) (OtherActor :type Actor%20Object%20Reference) (OtherComp :type Primitive%20Component%20Object%20Reference) (OtherBodyIndex :type Integer) (bFromSweep :type Boolean) (SweepResult :type Hit%20Result%20Structure%20%28by%20ref%29))
  ;[1 1 1] I Angrepssonen. Turret angriper og target lockon
  (Variables|Default|SetTarget OtherActor)
  (Variables|Default|SetTargeting true))

(event OnComponentEndOverlap(trigger)
  (params (OverlappedComponent :type Primitive%20Component%20Object%20Reference) (OtherActor :type Actor%20Object%20Reference) (OtherComp :type Primitive%20Component%20Object%20Reference) (OtherBodyIndex :type Integer))
  (Variables|Default|SetTargeting false))

(event Custom|updateTowerRotation
  (bind _tower1_gun (Variables|Default|GetTower1_Gun))
  (bind _target (Variables|Default|GetTarget))
  (bind _returnvalue (Transformation|GetActorLocation _target))
  (bind _returnvalue_2 (Transformation|GetWorldLocation _tower1_gun))
  (bind _returnvalue_3 (Math|Rotator|FindLookatRotation _returnvalue_2 _returnvalue))
  (bind (_roll _pitch _yaw) (Math|Rotator|BreakRotator _returnvalue_3))
  ;[1 1 1] Point turret to target
  (Transformation|SetWorldRotation (Variables|Default|GetTower1_Gun) (Math|Interpolation|RInterpTo (Transformation|GetWorldRotation (Variables|Default|GetTower1_Gun)) (Math|Rotator|MakeRotator 0.0 (Math|Float|ClampAngle _pitch -25.0 5e+01) _yaw) (Variables|Default|GetDeltaTime) 0.0) false false))

(event Custom|Idle
  (bind _tower1_gun (Variables|Default|GetTower1_Gun))
  (bind _returnvalue (Transformation|GetWorldRotation _tower1_gun))
  ;[1 1 1] Idle mode
  (Transformation|SetWorldRotation (Variables|Default|GetTower1_Gun) (Math|Interpolation|RInterpTo _returnvalue (Math|Rotator|MakeRotator 0.0 0.0 (+ (.Yaw (Math|Rotator|BreakRotator _returnvalue)) 1e+01)) (Variables|Default|GetDeltaTime) 5.0) false false))

(event Custom|Fire
  (Utilities|FlowControl|Delay 0.2)
  (Game|SpawnActorfromClass "/Game/Blueprints/Tower/Probe_BP.Probe_BP_C" (Transformation|GetSocketTransform (Variables|Default|GetTower1_Gun) "BarrelEnd" "RTS_World") "Undefined" 0 0))

(event EventBeginPlay)

(event Collision|EventActorBeginOverlap
  (params (OtherActor :type Actor%20Object%20Reference))
  ;[1 1 1] Point turret to target
)

(event EventTick
  (params (DeltaSeconds :type Float%20%28single-precision%29))
  ;[1 1 1] Kjør på tick
  (Variables|Default|SetDeltaTime DeltaSeconds)
  (if (Variables|Default|GetTargeting)
    (CallFunction|UpdateTowerRotation)
    (CallFunction|Fire)
    (else
      (CallFunction|Idle))))

(fn ConstructionScript)