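; Worm tower turret that turns toward and fires at actors entering its trigger volume.
; Overlap events store the latest actor as target and toggle targeting, which any exit clears.
; While targeting, Tick eases the mesh's yaw toward the target and spawns Probe_BP at the Fire socket, throttled by a short Delay.
; Otherwise, Tick calls a looping idle animation every frame.
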(event OnComponentBeginOverlap(Triggervolum)
  (params (OverlappedComponent :type Primitive%20Component%20Object%20Reference) (OtherActor :type Actor%20Object%20Reference) (OtherComp :type Primitive%20Component%20Object%20Reference) (OtherBodyIndex :type Integer) (bFromSweep :type Boolean) (SweepResult :type Hit%20Result%20Structure%20%28by%20ref%29))
  ;[1 1 1] Entering attack radius
  (Variables|Default|SetTarget OtherActor)
  (Variables|Default|SetTargeting? true))

(event OnComponentEndOverlap(Triggervolum)
  (params (OverlappedComponent :type Primitive%20Component%20Object%20Reference) (OtherActor :type Actor%20Object%20Reference) (OtherComp :type Primitive%20Component%20Object%20Reference) (OtherBodyIndex :type Integer))
  ;[1 1 1] Exiting attack radius
  (Variables|Default|SetTargeting? false))

(event Custom|UpdateTowerRotatoion
  ;[1 1 1] Aim at target
  (Transformation|SetWorldRotation (Variables|Default|GetWorm_Mesh) (Math|Interpolation|RInterpTo (Transformation|GetWorldRotation (Variables|Default|GetWorm_Mesh)) (Math|Rotator|MakeRotator 0.0 0.0 (.Yaw (Math|Rotator|BreakRotator (Math|Rotator|FindLookatRotation (Transformation|GetWorldLocation (Variables|Default|GetWorm_Mesh)) (Transformation|GetActorLocation (Variables|Default|GetTarget)))))) (Variables|Default|GetDeltaTime) 5.0) false false))

(event Custom|Idle
  ;[1 1 1] Idle worm
  (Components|Animation|PlayAnimation (Variables|Default|GetWorm_Mesh) "/Game/Mesh/Tower/Animations/Worm_Idle_Animation01a.Worm_Idle_Animation01a" true))

(event Custom|Fire%20turret
  (Utilities|FlowControl|Delay 0.2)
  (Game|SpawnActorfromClass "/Game/Blueprints/Tower/Probe_BP.Probe_BP_C" (Transformation|GetSocketTransform (Variables|Default|GetWorm_Mesh) "Fire" "RTS_World") "Undefined" 0 0))

(event EventTick
  (params (DeltaSeconds :type Float%20%28single-precision%29))
  ;[1 1 1] Execute tick
  (Variables|Default|SetDeltaTime DeltaSeconds)
  (if (Variables|Default|GetTargeting?)
    (CallFunction|UpdateTowerRotatoion)
    (CallFunction|FireTurret)
    (else
      (CallFunction|Idle))))

(fn ConstructionScript)