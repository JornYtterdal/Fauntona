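; Enemy Blueprint that attacks the player with line traces on a looping timer.
; StartAttacking runs Attack every AIAttack seconds until StopAttacking clears the timer.
; Attack traces on Visibility toward player 0 with debug drawing and damages whatever actor it hits.
; AnyDamage is empty; the Health reduction and death logic (unpossess, destroy) is disconnected, so it never runs.
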(event Custom|StopAttacking
  ;[1 1 1] Attack (if it worked)
  (Utilities|Time|ClearTimerbyFunctionName 0 "Attack"))

(event Custom|Attack
  ;[1 1 1] Attack (if it worked)
  (bind (_outhit _returnvalue) (Collision|LineTraceByChannel (Transformation|GetActorLocation) (Transformation|GetActorLocation (Game|GetPlayerCharacter 0)) "TraceTypeQuery1" false 0 "ForDuration"))
  (if _returnvalue
    (Game|Damage|ApplyDamage (.HitActor (Collision|BreakHitResult _outhit)) 1.0 0 0)))

(event Custom|StartAttacking
  ;[1 1 1] Attack (if it worked)
  (Utilities|Time|SetTimerbyFunctionName 0 "Attack" (Variables|Default|GetAI%20attack) true))

(event Game|Damage|EventAnyDamage
  (params (Damage :type Float%20%28single-precision%29) (DamageType :type Damage%20Type%20Object%20Reference) (InstigatedBy :type Controller%20Object%20Reference) (DamageCauser :type Actor%20Object%20Reference))
  ;[1 1 1] Health
)

(fn ConstructionScript)