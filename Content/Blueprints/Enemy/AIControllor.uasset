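; AI controller for Enemy pawns that runs the Ai_Brains behavior tree when it possesses one.
; AI perception updates about the FauntonaCharacter player write whether it is sensed into the CanSeePlayer blackboard key.
; A disconnected branch that called StartAttacking or StopAttacking on the controlled Enemy never runs, so this controller only feeds sight state to the tree.
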(event OnTargetPerceptionUpdated(AIPerception)
  (params (Actor :type Actor%20Object%20Reference) (Stimulus :type AI%20Stimulus%20Structure))
  (Utilities|Casting|CastToFauntonaCharacter Actor)
  (AI|Components|Blackboard|SetValueasBool (Variables|Default|GetBlackboard) (Utilities|Name|MakeLiteralName "CanSeePlayer") (.bSuccessfullySensed (Utilities|Struct|BreakAIStimulus Stimulus))))

(event EventOnPossess
  (params (PossessedPawn :type Pawn%20Object%20Reference))
  ;[1 1 1] Kjør Behaviour tree
  (Utilities|Casting|CastToEnemy PossessedPawn)
  (AI|RunBehaviorTree "/Game/Blueprints/Enemy/Ai_Brains.Ai_Brains"))

(fn ConstructionScript)